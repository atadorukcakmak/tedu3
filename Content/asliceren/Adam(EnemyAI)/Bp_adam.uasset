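; Enemy AI character that chases the player, with behavior switched by the IsikAcik (light on) flag.
; Each Tick, with the flag set, it pursues a player within a shorter range at the faster walk speed.
; Otherwise it uses a longer detection range but also requires line of sight, and moves at half that speed.
; Both branches share one AIMoveTo on the player, reissued every frame while conditions hold.
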(event `self.ReceiveTick`
  (params (DeltaSeconds :type "Float (single-precision)"))
  (bind _charactermovement (`self.CharacterMovement`))
  (if (`self.Isik acik?`)
    (if (< (`self.GetDistanceTo` (`GameplayStatics.GetPlayerCharacter` 0)) 1000.0)
      (set `CharacterMovementComponent.MaxWalkSpeed` 400.0 _charactermovement)
      (`|AIMoveTo` self (0.0 0.0 0.0) (`GameplayStatics.GetPlayerCharacter` 0) :!label _label))
    (elif (< (`self.GetDistanceTo` (`GameplayStatics.GetPlayerCharacter` 0)) 2000.0)
      (if (`Controller.LineOfSightTo` (`self.GetController`) (`GameplayStatics.GetPlayerCharacter` 0) (0.0 0.0 0.0) false)
        (set `CharacterMovementComponent.MaxWalkSpeed` 200.0 _charactermovement)
        (goto _label)))))

(fn `UserConstructionScript`)