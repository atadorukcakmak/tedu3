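; Sliding double door that opens and closes through two custom events, with no trigger logic of its own.
; kapidugmesibasildi (button pressed) swaps a material slot on Cube and plays a Timeline that lerps both door meshes apart along local X.
; kapikapaniyo (door closing) sets another material and plays a second timeline in reverse from its end to bring them back together.
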(event `self.ReceiveBeginPlay`)

(event `kapi dugmesi basildi`
  (`PrimitiveComponent.SetMaterialByName` (`self.Cube`) "Materiale.002" "/Game/Keycards/Okuyucu/Materiale_007.Materiale_007")
  (bind (_direction _newtrack_0) (`Timeline|Timeline`)
    (:`Update`
      (`SceneComponent.K2_SetRelativeLocation` (`self.SM_Door_right`) (`KismetMathLibrary.VLerp` (240.0 -50.0 0.0) (510.0 -50.0 0.0) _newtrack_0) false false)
      (`SceneComponent.K2_SetRelativeLocation` (`self.SM_Door_left`) (`KismetMathLibrary.VLerp` (-240.0 -50.0 0.0) (-510.0 -50.0 0.0) _newtrack_0) false false))))

(event `kapi kapaniyo`
  (`PrimitiveComponent.SetMaterialByName` (`self.Cube`) "Materiale.002" "/Game/Keycards/Okuyucu/Materiale_008.Materiale_008")
  (bind (_direction _newtrack_0) (`Timeline|Timeline_0` :!via `ReverseFromEnd`)
    (:`Update`
      (`SceneComponent.K2_SetRelativeLocation` (`self.SM_Door_right`) (`KismetMathLibrary.VLerp` (240.0 -50.0 0.0) (510.0 -50.0 0.0) _newtrack_0) false false)
      (`SceneComponent.K2_SetRelativeLocation` (`self.SM_Door_left`) (`KismetMathLibrary.VLerp` (-240.0 -50.0 0.0) (-510.0 -50.0 0.0) _newtrack_0) false false))))

(fn `UserConstructionScript`)