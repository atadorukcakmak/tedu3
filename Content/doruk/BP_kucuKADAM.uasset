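; Enemy character (the "small man") that reveals itself, plays a one-time spawn sound and chases the player to attack.
; A one-second looping timer checks the player's Fenerkullanımı (flashlight use) flag: if set, it sprints from any distance; otherwise it approaches slowly within range.
; On arrival it plays an attack montage and, if still close, calls the player's ProgressBar event.
; The ölüm event plays a death montage, then destroys the actor.
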(event `koşu kontrolü`
  (bind _returnvalue (`GameplayStatics.GetPlayerPawn` 0))
  (set `CharacterMovementComponent.MaxWalkSpeed` 400.0 (`self.CharacterMovement`))
  (bind _returnvalue_2 (`GameplayStatics.GetActorOfClass` "/Game/FirstPerson/Blueprints/BP_FirstPersonCharacter.BP_FirstPersonCharacter_C"))
  (if (`/Game/FirstPerson/Blueprints/BP_FirstPersonCharacter.fenerkullanımı` _returnvalue_2)
    (`SceneComponent.SetHiddenInGame` (`self.Mesh`) false false)
    (if (`self.dogumses`)
      (`GameplayStatics.PlaySound2D` "/Game/SFX/kucukdogdu.kucukdogdu" 1.0 1.0 0.0 null null)
      (set `self.dogumses` false))
    (set `CharacterMovementComponent.MaxWalkSpeed` 1000.0 (`self.CharacterMovement`))
    (`|AIMoveTo` self (0.0 0.0 0.0) (`GameplayStatics.GetPlayerPawn` 0) 15.0
      (:`OnSuccess`
        (`|PlayMontage` (`self.Mesh`) "/Game/Dilara/AnimMontage_Yaku.AnimMontage_Yaku"
          (:`OnNotifyEnd`
            (if (< (`KismetMathLibrary.Vector_Distance` (`self.K2_GetActorLocation`) (`self.K2_GetActorLocation` (`GameplayStatics.GetPlayerPawn` 0))) 200.0)
              (bind _returnvalue_3 (`GameplayStatics.GetActorOfClass` "/Game/FirstPerson/Blueprints/BP_FirstPersonCharacter.BP_FirstPersonCharacter_C"))
              (`GameplayStatics.PlaySound2D` "/Game/SFX/attacked.attacked" 1.0 1.0 0.0 null null)
              (`/Game/FirstPerson/Blueprints/BP_FirstPersonCharacter.ProgressBar` _returnvalue_3))))))
    (elif (< (`KismetMathLibrary.Vector_Distance` (`self.K2_GetActorLocation`) (`self.K2_GetActorLocation` _returnvalue)) 1500.0)
      (`SceneComponent.SetHiddenInGame` (`self.Mesh`) false false)
      (if (`self.dogumses`)
        (`GameplayStatics.PlaySound2D` "/Game/SFX/kucukdogdu.kucukdogdu" 1.0 1.0 0.0 null null)
        (set `self.dogumses` false))
      (set `CharacterMovementComponent.MaxWalkSpeed` 300.0 (`self.CharacterMovement`))
      (`|AIMoveTo` self (0.0 0.0 0.0) _returnvalue 15.0
        (:`OnSuccess`
          (`|PlayMontage` (`self.Mesh`) "/Game/Dilara/AnimMontage_Yaku.AnimMontage_Yaku"
            (:`then`
              (if (< (`KismetMathLibrary.Vector_Distance` (`self.K2_GetActorLocation`) (`self.K2_GetActorLocation` (`GameplayStatics.GetPlayerPawn` 0))) 200.0)
                (bind _returnvalue_4 (`GameplayStatics.GetActorOfClass` "/Game/FirstPerson/Blueprints/BP_FirstPersonCharacter.BP_FirstPersonCharacter_C"))
                (`GameplayStatics.PlaySound2D` "/Game/SFX/attacked.attacked" 1.0 1.0 0.0 null null)
                (`/Game/FirstPerson/Blueprints/BP_FirstPersonCharacter.ProgressBar` _returnvalue_4)))))))))

(event `self.ReceiveBeginPlay`
  (`KismetSystemLibrary.K2_SetTimerDelegate` (delegate `koşu kontrolü`) 1.0 true))

(event `ölüm`
  (`|PlayMontage` (`self.Mesh`) "/Game/Pumpkinhulk/AnimBP_Die.AnimBP_Die"
    (:`OnCompleted`
      (`self.K2_DestroyActor`))))

(fn `IsAttacking`
  (returns (ReturnValue :type Boolean))
  (return (`AnimInstance.Montage_IsPlaying` (`SkeletalMeshComponent.GetAnimInstance` (`self.Mesh`)) null)))

(fn `IsWithinRange`
  (returns (ReturnValue :type Boolean))
  (return (< (`self.GetDistanceTo` (`GameplayStatics.GetPlayerCharacter` 0)) (`self.AttackRange`))))

(fn `UserConstructionScript`)