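; Enemy AI character "adam" that hunts the first-person player, reacting to flashlight use.
; A looping one-second timer from BeginPlay polls the player's Fenerkullanımı flag.
; When set, the enemy unhides, plays a sound and sprints via AIMoveTo at any range; otherwise it chases more slowly within range, with sound gated by Dogmases.
; On arrival it plays a montage, then calls the player's ProgressBar if still close.
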(event `koşu kontrolü`
  (bind _returnvalue (`GameplayStatics.GetPlayerPawn` 0))
  (set `CharacterMovementComponent.MaxWalkSpeed` 300.0 (`self.CharacterMovement`))
  (bind _returnvalue_2 (`GameplayStatics.GetActorOfClass` "/Game/FirstPerson/Blueprints/BP_FirstPersonCharacter.BP_FirstPersonCharacter_C"))
  (if (`/Game/FirstPerson/Blueprints/BP_FirstPersonCharacter.fenerkullanımı` _returnvalue_2)
    (`SceneComponent.SetHiddenInGame` (`self.Mesh`) false false)
    (`GameplayStatics.PlaySound2D` "/Game/SFX/kucukdogdu.kucukdogdu" 1.0 1.0 0.0 null null)
    (set `CharacterMovementComponent.MaxWalkSpeed` 800.0 (`self.CharacterMovement`))
    (`|AIMoveTo` self (0.0 0.0 0.0) (`GameplayStatics.GetPlayerPawn` 0) 50.0
      (:`OnSuccess`
        (`|PlayMontage` (`self.Mesh`) "/Game/Dilara/AnimMontage_Yaku.AnimMontage_Yaku"
          (:`then`
            (if (< (`KismetMathLibrary.Vector_Distance` (`self.K2_GetActorLocation`) (`self.K2_GetActorLocation` (`GameplayStatics.GetPlayerPawn` 0))) 200.0)
              (bind _returnvalue_3 (`GameplayStatics.GetActorOfClass` "/Game/FirstPerson/Blueprints/BP_FirstPersonCharacter.BP_FirstPersonCharacter_C"))
              (`/Game/FirstPerson/Blueprints/BP_FirstPersonCharacter.ProgressBar` _returnvalue_3))))))
    (elif (< (`KismetMathLibrary.Vector_Distance` (`self.K2_GetActorLocation`) (`self.K2_GetActorLocation` _returnvalue)) 1500.0)
      (`SceneComponent.SetHiddenInGame` (`self.Mesh`) false false)
      (if (`self.dogmases`)
        (`GameplayStatics.PlaySound2D` "/Game/SFX/kucukdogdu.kucukdogdu" 1.0 1.0 0.0 null null))
      (set `CharacterMovementComponent.MaxWalkSpeed` 375.0 (`self.CharacterMovement`))
      (`|AIMoveTo` self (0.0 0.0 0.0) _returnvalue 50.0
        (:`OnSuccess`
          (`|PlayMontage` (`self.Mesh`) "/Game/Dilara/AnimMontage_Yaku.AnimMontage_Yaku"
            (:`then`
              (if (< (`KismetMathLibrary.Vector_Distance` (`self.K2_GetActorLocation`) (`self.K2_GetActorLocation` (`GameplayStatics.GetPlayerPawn` 0))) 200.0)
                (bind _returnvalue_4 (`GameplayStatics.GetActorOfClass` "/Game/FirstPerson/Blueprints/BP_FirstPersonCharacter.BP_FirstPersonCharacter_C"))
                (`/Game/FirstPerson/Blueprints/BP_FirstPersonCharacter.ProgressBar` _returnvalue_4)))))))))

(event `self.ReceiveBeginPlay`
  (`KismetSystemLibrary.K2_SetTimerDelegate` (delegate `koşu kontrolü`) 1.0 true))

(fn `UserConstructionScript`)